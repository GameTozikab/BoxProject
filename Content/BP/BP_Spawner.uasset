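; BP_Spawner spawns a square grid of actors of the Actor class, Count per side, when play begins.
; Spacing derives from LFloat divided by Count, scaled by the spawner's X scale and truncated to whole units.
; Nested loops lay the grid out in the world X-Z plane from the root's location, shrinking each actor's scale in proportion to the spawner's scale and Count.
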(event EventBeginPlay
  (bind _self self)
  (bind _defaultsceneroot (Variables|Default|GetDefaultSceneRoot _self))
  (bind _returnvalue (Transformation|GetWorldLocation _defaultsceneroot))
  ;[1 1 1] Растояние между объектами
  (Variables|Default|SetL_Float (* (/ (Variables|Default|GetL_Float) (Math|Conversions|ToFloat(Integer) (Variables|Default|GetCount))) (/ (.x (.scale (Transformation|GetActorTransform self))) 1e+01)))
  ;[1 1 1] Появление объектов в заданном количестве
  (Variables|Default|SetNewVar_0 (* (Variables|Default|GetNewVar_0) 1.0))
  (for _index (range 0 (- (Variables|Default|GetCount) 1))
    (for _index_2 (range 0 (- (Variables|Default|GetCount) 1))
      (Game|SpawnActorfromClass (Variables|Default|GetActor) (Math|Transform|MakeTransform (Math|Vector|MakeVector (+ (Math|Conversions|ToFloat(Integer) (* _index_2 (Math|Float|Truncate (Variables|Default|GetL_Float)))) (.x _returnvalue)) (.y _returnvalue) (+ (.z _returnvalue) (Math|Conversions|ToFloat(Integer) (* _index (Math|Float|Truncate (Variables|Default|GetL_Float)))))) "0, 0, 0" (/ (/ (.scale (Transformation|GetActorTransform self)) (Math|Conversions|ToFloat(Integer) (Variables|Default|GetCount))) 3.0)) "Undefined" 0 0))))

(fn ConstructionScript)
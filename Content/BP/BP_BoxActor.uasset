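; BP_BoxActor is a box that reacts to damage by briefly swapping its cube material and passing damage to neighbors in a chain reaction.
; Damage of exactly 5 always triggers it, while other damage triggers it only when the Check flag is set.
; After short delays, scale-adjusted line traces along world ±X and ±Z apply damage to hit actors.
; Check clears on trigger and resets after a cooldown, limiting re-triggering.
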(event EventBeginPlay
  (Rendering|Material|SetMaterial (Variables|Default|GetCube) 0 "/Engine/BasicShapes/BasicShapeMaterial.BasicShapeMaterial"))

(event Collision|EventActorBeginOverlap
  (params (OtherActor :type Actor%20Object%20Reference)))

(event EventTick
  (params (DeltaSeconds :type Float%20%28single-precision%29)))

(event Game|Damage|EventAnyDamage
  (params (Damage :type Float%20%28single-precision%29) (DamageType :type Damage%20Type%20Object%20Reference) (InstigatedBy :type Controller%20Object%20Reference) (DamageCauser :type Actor%20Object%20Reference))
  (bind _self self)
  (bind _b (Variables|Default|GetB))
  (bind _returnvalue (Transformation|GetActorTransform _self))
  (bind _returnvalue_2 (* _b (.z (.scale _returnvalue))))
  (bind _returnvalue_3 (* _b (.x (.scale _returnvalue))))
  (if (== Damage 5.0)
    ;[1 1 1] Смена материала
    (Rendering|Material|SetMaterial (Variables|Default|GetCube) 0 "/Engine/MapTemplates/Materials/BasicAsset01.BasicAsset01" :!label _label)
    (Variables|Default|SetCheck false)
    (Utilities|FlowControl|Delay 1.0)
    (Rendering|Material|SetMaterial (Variables|Default|GetCube) 0 "/Engine/BasicShapes/BasicShapeMaterial.BasicShapeMaterial")
    (Utilities|FlowControl|Delay 0.2)
    (Utilities|FlowControl|Sequence
      (:then_0
        ;[1 1 1] Запуск луча
        (CallFunction|TraceX (* _returnvalue_3 -1.0))
        (CallFunction|TraceX _returnvalue_3))
      (:then_1
        (CallFunction|TraceZ (* _returnvalue_2 -1.0))
        (CallFunction|TraceZ _returnvalue_2)))
    (Utilities|FlowControl|Delay 4.0)
    (Variables|Default|SetCheck true)
    (elif (Variables|Default|GetCheck)
      (goto _label))))

(fn ConstructionScript)

(fn TraceX
  (params (B :type Float%20%28single-precision%29))
  (bind _cube (Variables|Default|GetCube))
  (bind _returnvalue (Transformation|GetWorldLocation _cube))
  (bind (_outhit _returnvalue_2) (Collision|LineTraceByChannel (Transformation|GetWorldLocation _cube) (Math|Vector|MakeVector (+ (.x _returnvalue) B) (.y _returnvalue) (.z _returnvalue)) "TraceTypeQuery1" true 0 "None"))
  (if _returnvalue_2
    (Game|Damage|ApplyDamage (.HitActor (Collision|BreakHitResult _outhit)) 1e+01 0 0 "/Script/Engine.DamageType")))

(fn TraceZ
  (params (B :type Float%20%28single-precision%29))
  (bind _cube (Variables|Default|GetCube))
  (bind _returnvalue (Transformation|GetWorldLocation _cube))
  (bind (_outhit _returnvalue_2) (Collision|LineTraceByChannel (Transformation|GetWorldLocation _cube) (Math|Vector|MakeVector (.x _returnvalue) (.y _returnvalue) (+ (.z _returnvalue) B)) "TraceTypeQuery1" false 0 "None"))
  (if _returnvalue_2
    (Game|Damage|ApplyDamage (.HitActor (Collision|BreakHitResult _outhit)) 1e+01 0 0 "/Script/Engine.DamageType")))